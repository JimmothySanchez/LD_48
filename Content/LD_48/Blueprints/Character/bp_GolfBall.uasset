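; Physics-driven golf ball actor that damages what it hits and can display a predicted trajectory.
; Each tick moves the actor to the Sphere's location and uses a sphere trace to switch between frictional and standard linear damping.
; Hits damage destructible components and actors, playing a speed-gated sound throttled by a DoOnce with a randomized reset timer.
; Trajectory functions draw a supplied path prediction as instanced meshes, or clear it.
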(event `self.ReceiveBeginPlay`)

(event `self.ReceiveTick`
  (params (DeltaSeconds :type "Float (single-precision)"))
  (`self.K2_SetActorLocation` (`SceneComponent.K2_GetComponentLocation` (`self.Sphere`)) true)
  (`self.UpdateFriction`))

(event `self.Sphere.OnComponentHit`
  (params (HitComponent :type "PrimitiveComponent Object Reference") (OtherActor :type "Actor Object Reference") (OtherComp :type "PrimitiveComponent Object Reference") (NormalImpulse :type "Vector Structure") (Hit :type "HitResult Structure (by ref)"))
  (bind (_bblockinghit _binitialoverlap _time _distance _location _impactpoint _normal) (`GameplayStatics.BreakHitResult` Hit))
  (`|ExecutionSequence`
    (:`then_0`
      ;[1 1 1] Damage
      (bind _asdestructible_component (cast `DestructibleComponent` OtherComp))
      (`DestructibleComponent.ApplyDamage` _asdestructible_component 100.0 _location NormalImpulse (`KismetMathLibrary.VSize` _normal))
      (`GameplayStatics.ApplyDamage` OtherActor 100.0))
    (:`then_1`
      (if (> (`KismetMathLibrary.VSize` (`SceneComponent.GetComponentVelocity` (`self.Sphere`))) 100.0)
        (`/Engine/EditorBlueprintResources/StandardMacros.DoOnce` false :!label _label
          (:`Completed`
            (`GameplayStatics.PlaySoundAtLocation` "/Game/LD_48/Audio/Effects/Hit_Cue.Hit_Cue" (`.ImpactPoint` (`GameplayStatics.BreakHitResult` Hit)) (struct) 1.0 1.0 0.0 null null null)
            (`KismetSystemLibrary.K2_SetTimerDelegate` (delegate `CustomEvent_0`) (`KismetMathLibrary.RandomFloatInRange` 0.1 0.2))))))))

(event `CustomEvent_0`
  (goto _label :!via `Reset`))

(fn `ClearTrajectoryVisuals`
  (`InstancedStaticMeshComponent.ClearInstances` (`self.InstancedStaticMesh`)))

(fn `UpdateFriction`
  (bind _returnvalue (`SceneComponent.K2_GetComponentLocation` (`self.Sphere`)))
  (bind (_outhit _returnvalue_2) (`KismetSystemLibrary.SphereTraceSingle` _returnvalue _returnvalue 52.0 "TraceTypeQuery1"))
  (if _returnvalue_2
    (`PrimitiveComponent.SetLinearDamping` (`self.Sphere`) (`self.FrictionalDrag`))
    (else
      (`PrimitiveComponent.SetLinearDamping` (`self.Sphere`) (`self.StandardDrag`)))))

(fn `UpdateTrajectoryVisuals`
  (params (Prediction :type "PredictProjectilePathResult Structure"))
  (`InstancedStaticMeshComponent.ClearInstances` (`self.InstancedStaticMesh`))
  (for (_array_element _array_index) (`.PathData` (break `PredictProjectilePathResult` Prediction))
    (if (> _array_index 1)
      (`InstancedStaticMeshComponent.AddInstanceWorldSpace` (`self.InstancedStaticMesh`) (`KismetMathLibrary.MakeTransform` (`.Location` (break `PredictProjectilePathPointData` _array_element)) (struct) (0.25 0.25 0.25))))))

(fn `UserConstructionScript`)