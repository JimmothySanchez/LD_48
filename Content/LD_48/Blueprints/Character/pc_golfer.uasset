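; Player controller for a physics golf game, handling HUD, right-mouse camera look, limited strokes and the win screen.
; Aim and force functions set up the shot; Launch applies it as the bp_GolfBall's physics velocity and spends a stroke.
; Tick draws a predicted projectile path while the ball rests with strokes left.
; Once strokes run out and the ball stops, a timer reloads the level unless movement or winning cancels it.
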(event `self.ReceiveBeginPlay`
  (set `self.StrokeCount` (`self.InitialStrokecount`))
  (bind _returnvalue (`|CreateWidget` "/Game/LD_48/Blueprints/UI/wdg_HUD.wdg_HUD_C"))
  (set `self.HUD` _returnvalue)
  (`UserWidget.AddToPlayerScreen` _returnvalue 0)
  (`WidgetBlueprintLibrary.SetInputMode_GameAndUIEx` self _returnvalue "DoNotLock" false)
  (set `self.bShowMouseCursor` true))

(event `self.ReceiveTick`
  (params (DeltaSeconds :type "Float (single-precision)"))
  (`self.UpdateIsMoving`)
  (`self.EstimateTrajectory`))

(event `InputAction|Exit`
  (params (Key :type "Key Structure"))
  (:`Pressed`
    (`KismetSystemLibrary.QuitGame` null "Quit")))

(event `InputAxisKey|MouseX`
  (params (AxisValue :type "Float (single-precision)"))
  ;[1 1 1] Camera controls
  (if (`self.HasCameraControl`)
    (`self.AddYawInput` (* AxisValue (`self.Camera Speed`)))))

(event `InputAxisKey|MouseY`
  (params (AxisValue :type "Float (single-precision)"))
  ;[1 1 1] Camera controls
  (if (`self.HasCameraControl`)
    (`self.AddPitchInput` (* (* AxisValue (`self.Camera Speed`)) -1.0))))

(event `Key|RightMouseButton`
  (params (Key :type "Key Structure"))
  (:`Pressed`
    (set `self.HasCameraControl` true))
  (:`Released`
    (set `self.HasCameraControl` false)))

(event `PlayerWins`
  (set `self.Won` true)
  (`Widget.RemoveFromParent` (`self.HUD`))
  (`KismetSystemLibrary.K2_ClearAndInvalidateTimerHandle` (`self.EndGameTimer`))
  (bind _returnvalue (`|CreateWidget` "/Game/LD_48/Blueprints/UI/wdg_Win.wdg_Win_C"))
  (`UserWidget.AddToPlayerScreen` _returnvalue 0))

(fn `EstimateTrajectory`
  (locals (GolfBall :type "/Game/LD_48/Blueprints/Character/bp_GolfBall Object Reference"))
  (bind _golfball (`local.GolfBall`))
  (bind _asbp_golf_ball (cast `/Game/LD_48/Blueprints/Character/bp_GolfBall` (`self.K2_GetPawn`)))
  (set `local.GolfBall` _asbp_golf_ball)
  (if (or (`self.IsMoving`) (< (`self.StrokeCount`) 1) (`self.Won`))
    (`/Game/LD_48/Blueprints/Character/bp_GolfBall.ClearTrajectoryVisuals` (`local.GolfBall`))
    (else
      (bind _predictresult (`GameplayStatics.Blueprint_PredictProjectilePath_Advanced` (make `PredictProjectilePathParams` :`StartLocation` (`self.K2_GetActorLocation` _golfball) :`LaunchVelocity` (* (`SceneComponent.GetForwardVector` (`/Game/LD_48/Blueprints/Character/bp_GolfBall.PotentialRot` _asbp_golf_ball)) (`self.Potential Force`)) :`bTraceWithCollision` true :`ProjectileRadius` 49.0 :`TraceChannel` "ECC_PhysicsBody" :`ActorsToIgnore` (`|MakeArray` _golfball :!type "Actor Object Reference") :`bTraceComplex` true)))
      (`/Game/LD_48/Blueprints/Character/bp_GolfBall.UpdateTrajectoryVisuals` (`local.GolfBall`) _predictresult))))

(fn `Launch`
  (bind _asbp_golf_ball (cast `/Game/LD_48/Blueprints/Character/bp_GolfBall` (`self.K2_GetPawn`)))
  (`PrimitiveComponent.SetPhysicsLinearVelocity` (`/Game/LD_48/Blueprints/Character/bp_GolfBall.Sphere` _asbp_golf_ball) (* (`SceneComponent.GetForwardVector` (`/Game/LD_48/Blueprints/Character/bp_GolfBall.PotentialRot` _asbp_golf_ball)) (`self.Potential Force`)) false "None")
  (`/Engine/EditorBlueprintResources/StandardMacros.DecrementInt` (`self.StrokeCount`)
    (:`  `
      (`GameplayStatics.PlaySoundAtLocation` "/Game/LD_48/Audio/Effects/Pickup_Cue.Pickup_Cue" (`self.K2_GetActorLocation` _asbp_golf_ball) (struct) 1.0 1.0 0.0 null null null))))

(fn `RestartMap`
  (bind _returnvalue (`GameplayStatics.GetCurrentLevelName` true))
  (`GameplayStatics.OpenLevel` (`KismetStringLibrary.Conv_StringToName` _returnvalue)))

(fn `Rotate_Right`
  (params (NewParam :type "Float (double-precision)"))
  (bind _asbp_golf_ball (cast `/Game/LD_48/Blueprints/Character/bp_GolfBall` (`self.K2_GetPawn`)))
  (`SceneComponent.K2_AddRelativeRotation` (`/Game/LD_48/Blueprints/Character/bp_GolfBall.PotentialRot` _asbp_golf_ball) (`KismetMathLibrary.MakeRotator` 0.0 0.0 NewParam) false false))

(fn `Rotate_Up`
  (params (NewParam :type "Float (double-precision)"))
  (bind _asbp_golf_ball (cast `/Game/LD_48/Blueprints/Character/bp_GolfBall` (`self.K2_GetPawn`)))
  (`SceneComponent.K2_AddRelativeRotation` (`/Game/LD_48/Blueprints/Character/bp_GolfBall.PotentialRot` _asbp_golf_ball) (`KismetMathLibrary.MakeRotator` 0.0 NewParam) false false))

(fn `UpdateIsMoving`
  (if (not (`self.Won`))
    (bind _asbp_golf_ball (cast `/Game/LD_48/Blueprints/Character/bp_GolfBall` (`self.K2_GetPawn`)))
    (set `self.IsMoving` (> (`KismetMathLibrary.VSize` (`SceneComponent.GetComponentVelocity` (`/Game/LD_48/Blueprints/Character/bp_GolfBall.Sphere` _asbp_golf_ball))) 10.0))
    (if (`self.IsMoving`)
      (if (`KismetSystemLibrary.K2_IsValidTimerHandle` (`self.EndGameTimer`))
        (`KismetSystemLibrary.K2_ClearAndInvalidateTimerHandle` (`self.EndGameTimer`)))
      (elif (and (<= (`self.StrokeCount`) 0) (not (`KismetSystemLibrary.K2_IsValidTimerHandle` (`self.EndGameTimer`))))
        (bind _returnvalue (`KismetSystemLibrary.K2_SetTimer` null "RestartMap" (`self.FinalRestDurration`)))
        (set `self.EndGameTimer` _returnvalue)))))

(fn `UserConstructionScript`)

(fn `VelocityUp`
  (params (Velocity :type "Float (double-precision)"))
  (set `self.Potential Force` (`KismetMathLibrary.FClamp` (+ (* Velocity (`self.PotentialForceIncrement`)) (`self.Potential Force`)) (`self.Potential Force_Min`) (`self.Potential Force_Max`))))