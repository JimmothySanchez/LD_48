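; Explosive barrel actor that blows up the first time it takes any damage.
; A DoOnce gate on AnyDamage fires the RadialForce impulse, then spawns a Niagara explosion, a light flash actor and an explosion sound at that component's location.
; The graph neither applies damage nor destroys the barrel afterward.
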(event `self.ReceiveAnyDamage`
  (params (Damage :type "Float (single-precision)") (DamageType :type "DamageType Object Reference") (InstigatedBy :type "Controller Object Reference") (DamageCauser :type "Actor Object Reference"))
  (`/Engine/EditorBlueprintResources/StandardMacros.DoOnce` false
    (:`Completed`
      (`RadialForceComponent.FireImpulse` (`self.RadialForce`))
      (`NiagaraFunctionLibrary.SpawnSystemAtLocation` "/Game/LD_48/Particles/ns_BarrelExplosion.ns_BarrelExplosion" (`SceneComponent.K2_GetComponentLocation` (`self.RadialForce`)) (struct) (3.0 3.0 3.0))
      (`|SpawnActorFromClass` "/Game/LD_48/Blueprints/Actors/bp_LightFlash.bp_LightFlash_C" (`KismetMathLibrary.MakeTransform` (`SceneComponent.K2_GetComponentLocation` (`self.RadialForce`))) "Undefined" "OverrideRootScale" null null)
      (`GameplayStatics.PlaySoundAtLocation` "/Game/LD_48/Audio/Effects/Explosion_Cue.Explosion_Cue" (`SceneComponent.K2_GetComponentLocation` (`self.RadialForce`)) (struct) 1.0 1.0 0.0 null null null))))

(fn `UserConstructionScript`)