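; bp_1UP is an actor that shows a Wdg_1Stroke screen widget tracking its location in the world.
; On BeginPlay it creates the widget and adds it to the player screen, then removes it when destroyed.
; Each Tick it projects the actor location to screen space, repositioning the widget or hiding it when projection fails.
; It contains no overlap or pickup logic of its own.
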(event `self.ReceiveBeginPlay`
  (bind _returnvalue (`|CreateWidget` "/Game/LD_48/Blueprints/UI/wdg_1Stroke.wdg_1Stroke_C"))
  (set `self.WidgetRef` _returnvalue)
  (`UserWidget.AddToPlayerScreen` _returnvalue 0))

(event `self.ReceiveTick`
  (params (DeltaSeconds :type "Float (single-precision)"))
  (bind _widgetref (`self.WidgetRef`))
  (bind (_screenposition _returnvalue) (`WidgetLayoutLibrary.ProjectWorldLocationToWidgetPosition` (`GameplayStatics.GetPlayerController` 0) (`self.K2_GetActorLocation`)))
  (if _returnvalue
    (`Widget.SetVisibility` _widgetref "Visible")
    (`UserWidget.SetPositionInViewport` _widgetref _screenposition true)
    (else
      (`Widget.SetVisibility` _widgetref "Hidden"))))

(event `self.ReceiveDestroyed`
  (`Widget.RemoveFromParent` (`self.WidgetRef`)))

(fn `UserConstructionScript`)